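; BP_SceneBox builds and runs the board for a 2048-style slime merge puzzle.
; On BeginPlay it spawns a centered tile grid, lines all four sides with bubble guns, then generates a slime on a random empty tile.
; MergeSlimes takes two slime rows, merges equal-energy neighbors by doubling or DT_SlimeMerge recipes, and snaps survivors to target transforms.
; It then calls turn alternation, triggers merged slimes and generates another slime.
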(event EventBeginPlay
  (|CreateTile
    (:Completed
      (|CreateBubbleGun
        (:Completed
          (CallFunction|GenerateSlime))))))

(fn ConstructionScript)

(fn MergeSlimes
  (params (B1A_S :type Array%20of%20BP%20Slime%20Object%20References) (B1A_T :type Array%20of%20BP%20Floor%20Tile%20Object%20References) (B2A_S :type Array%20of%20BP%20Slime%20Object%20References) (B2A_T :type Array%20of%20BP%20Floor%20Tile%20Object%20References))
  (LocalVariables|SetS1 B1A_S)
  (LocalVariables|SetT1 B1A_T)
  (LocalVariables|SetS2 B2A_S)
  (LocalVariables|SetT2 B2A_T)
  (Utilities|Set|Clear (Variables|Default|GetMergedSlime))
  (Utilities|Merge (LocalVariables|GetS1)
    (:Completed
      (for (_array_element _array_index) (LocalVariables|GetS1)
        (Transformation|SetActorTransform _array_element (Transformation|GetActorTransform (Utilities|Array|Get(acopy) (LocalVariables|GetT1) _array_index))))
      (Utilities|Merge (LocalVariables|GetS2)
        (:Completed
          (for (_array_element_2 _array_index_2) (LocalVariables|GetS2)
            (Transformation|SetActorTransform _array_element_2 (Transformation|GetActorTransform (Utilities|Array|Get(acopy) (LocalVariables|GetT2) _array_index_2))))
          (Default|CallTurnAlternation)
          (bind _result (Utilities|Set|ToArray (Variables|Default|GetMergedSlime)))
          (for _array_element_3 _result
            (Default|Meger _array_element_3))
          (CallFunction|GenerateSlime))))))

(fn GenerateSlime
  (bind _floortile_empty (Variables|Default|GetFloorTile_Empty))
  (bind _outitem (Utilities|Array|Random _floortile_empty))
  (Utilities|SelectEmptyTiles
    (:Completed
      (Utilities|IsValid _outitem
        (:Is%20Valid
          (Default|GenerateSlime _outitem (Variables|Default|GetAdvancedMode?)))))))