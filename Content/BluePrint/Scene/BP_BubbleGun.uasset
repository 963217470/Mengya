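; BP_BubbleGun is a clickable scene actor that triggers slime merging, showing a highlight Cube while the cursor hovers.
; When BP_SceneBox's Click flag is set, a click gathers overlapping BP_Slime and BP_FloorTile actors from Box1 and Box2.
; An exchange sort orders each list farthest-first from the gun.
; The lists go to BP_SceneBox's MergeSlimes with an axis flag derived from the gun's right vector.
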(event OnClicked(Cube)
  (params (TouchedComponent :type Primitive%20Component%20Object%20Reference) (ButtonPressed :type Key%20Structure :default "None"))
  (bind _returnvalue (Actor|GetActorOfClass "/Game/BluePrint/Scene/BP_SceneBox.BP_SceneBox_C"))
  (if (Variables|/Game/BluePrint/Scene/BP_SceneBox.BP_SceneBox_C|GetClick _returnvalue)
    (Utilities|Array|Clear (Variables|Default|GetB1A%20S))
    (Utilities|Array|Clear (Variables|Default|GetB1A%20T))
    (Utilities|Array|Clear (Variables|Default|GetB2A%20S))
    (Utilities|Array|Clear (Variables|Default|GetB2A%20T))
    (bind _output_get (Variables|Default|SetB1A_S (Collision|GetOverlappingActors (Variables|Default|GetBox1) "/Game/BluePrint/Slime/BP_Slime.BP_Slime_C" :!class /Script/Engine.PrimitiveComponent)))
    (Utilities|Sort _output_get
      (:Completed
        (bind _output_get_2 (Variables|Default|SetB2A_S (Collision|GetOverlappingActors (Variables|Default|GetBox2) "/Game/BluePrint/Slime/BP_Slime.BP_Slime_C" :!class /Script/Engine.PrimitiveComponent)))
        (Utilities|Sort _output_get_2
          (:Completed
            (bind _output_get_3 (Variables|Default|SetB1A_T (Collision|GetOverlappingActors (Variables|Default|GetBox1) "/Game/BluePrint/Scene/BP_FloorTile.BP_FloorTile_C" :!class /Script/Engine.PrimitiveComponent)))
            (Utilities|Sort _output_get_3
              (:Completed
                (bind _output_get_4 (Variables|Default|SetB2A_T (Collision|GetOverlappingActors (Variables|Default|GetBox2) "/Game/BluePrint/Scene/BP_FloorTile.BP_FloorTile_C" :!class /Script/Engine.PrimitiveComponent)))
                (Utilities|Sort _output_get_4
                  (:Completed
                    (bind _returnvalue_2 (Actor|GetActorOfClass "/Game/BluePrint/Scene/BP_SceneBox.BP_SceneBox_C"))
                    (Utilities|IsValid _returnvalue_2
                      (:Is%20Valid
                        (for _array_element (Variables|Default|GetB1A_S)
                          (bind _asbp_slime (Utilities|Casting|CastToBP_Slime _array_element))
                          (Utilities|Array|Add (Variables|Default|GetB1A%20S) _asbp_slime))
                        (for _array_element_2 (Variables|Default|GetB2A_S)
                          (bind _asbp_slime_2 (Utilities|Casting|CastToBP_Slime _array_element_2))
                          (Utilities|Array|Add (Variables|Default|GetB2A%20S) _asbp_slime_2))
                        (for _array_element_3 (Variables|Default|GetB1A_T)
                          (bind _asbp_floor_tile (Utilities|Casting|CastToBP_FloorTile _array_element_3))
                          (Utilities|Array|Add (Variables|Default|GetB1A%20T) _asbp_floor_tile))
                        (for _array_element_4 (Variables|Default|GetB2A_T)
                          (bind _asbp_floor_tile_2 (Utilities|Casting|CastToBP_FloorTile _array_element_4))
                          (Utilities|Array|Add (Variables|Default|GetB2A%20T) _asbp_floor_tile_2))
                        (Default|MergeSlimes _returnvalue_2 (Variables|Default|GetB1A%20S) (Variables|Default|GetB1A%20T) (Variables|Default|GetB2A%20S) (Variables|Default|GetB2A%20T) (== (Math|Float|Absolute(Float) (.x (Math|Vector|Normalize (Math|Vector|GetRightVector (Variables|Default|GetDefaultSceneRoot)) 1.0))) 0.0))))))))))))
    (else
      (Development|PrintString "Hello"))))

(event OnBeginCursorOver(Cube)
  (params (TouchedComponent :type Primitive%20Component%20Object%20Reference))
  (Rendering|SetVisibility (Variables|Default|GetCube) true false))

(event OnEndCursorOver(Cube)
  (params (TouchedComponent :type Primitive%20Component%20Object%20Reference))
  (Rendering|SetVisibility (Variables|Default|GetCube) false false))

(event OnBeginCursorOver(泡泡机模型_1_)
  (params (TouchedComponent :type Primitive%20Component%20Object%20Reference))
  (Rendering|SetVisibility (Variables|Default|GetCube) true false))

(event OnEndCursorOver(泡泡机模型_1_)
  (params (TouchedComponent :type Primitive%20Component%20Object%20Reference))
  (Rendering|SetVisibility (Variables|Default|GetCube) false false))

(event OnClicked(泡泡机模型_1_)
  (params (TouchedComponent :type Primitive%20Component%20Object%20Reference) (ButtonPressed :type Key%20Structure :default "None"))
  (bind _returnvalue (Actor|GetActorOfClass "/Game/BluePrint/Scene/BP_SceneBox.BP_SceneBox_C"))
  (if (Variables|/Game/BluePrint/Scene/BP_SceneBox.BP_SceneBox_C|GetClick _returnvalue)
    (Utilities|Array|Clear (Variables|Default|GetB1A%20S))
    (Utilities|Array|Clear (Variables|Default|GetB1A%20T))
    (Utilities|Array|Clear (Variables|Default|GetB2A%20S))
    (Utilities|Array|Clear (Variables|Default|GetB2A%20T))
    (bind _output_get (Variables|Default|SetB1A_S (Collision|GetOverlappingActors (Variables|Default|GetBox1) "/Game/BluePrint/Slime/BP_Slime.BP_Slime_C" :!class /Script/Engine.PrimitiveComponent)))
    (Utilities|Sort _output_get
      (:Completed
        (bind _output_get_2 (Variables|Default|SetB2A_S (Collision|GetOverlappingActors (Variables|Default|GetBox2) "/Game/BluePrint/Slime/BP_Slime.BP_Slime_C" :!class /Script/Engine.PrimitiveComponent)))
        (Utilities|Sort _output_get_2
          (:Completed
            (bind _output_get_3 (Variables|Default|SetB1A_T (Collision|GetOverlappingActors (Variables|Default|GetBox1) "/Game/BluePrint/Scene/BP_FloorTile.BP_FloorTile_C" :!class /Script/Engine.PrimitiveComponent)))
            (Utilities|Sort _output_get_3
              (:Completed
                (bind _output_get_4 (Variables|Default|SetB2A_T (Collision|GetOverlappingActors (Variables|Default|GetBox2) "/Game/BluePrint/Scene/BP_FloorTile.BP_FloorTile_C" :!class /Script/Engine.PrimitiveComponent)))
                (Utilities|Sort _output_get_4
                  (:Completed
                    (bind _returnvalue_2 (Actor|GetActorOfClass "/Game/BluePrint/Scene/BP_SceneBox.BP_SceneBox_C"))
                    (Utilities|IsValid _returnvalue_2
                      (:Is%20Valid
                        (for _array_element (Variables|Default|GetB1A_S)
                          (bind _asbp_slime (Utilities|Casting|CastToBP_Slime _array_element))
                          (Utilities|Array|Add (Variables|Default|GetB1A%20S) _asbp_slime))
                        (for _array_element_2 (Variables|Default|GetB2A_S)
                          (bind _asbp_slime_2 (Utilities|Casting|CastToBP_Slime _array_element_2))
                          (Utilities|Array|Add (Variables|Default|GetB2A%20S) _asbp_slime_2))
                        (for _array_element_3 (Variables|Default|GetB1A_T)
                          (bind _asbp_floor_tile (Utilities|Casting|CastToBP_FloorTile _array_element_3))
                          (Utilities|Array|Add (Variables|Default|GetB1A%20T) _asbp_floor_tile))
                        (for _array_element_4 (Variables|Default|GetB2A_T)
                          (bind _asbp_floor_tile_2 (Utilities|Casting|CastToBP_FloorTile _array_element_4))
                          (Utilities|Array|Add (Variables|Default|GetB2A%20T) _asbp_floor_tile_2))
                        (Default|MergeSlimes _returnvalue_2 (Variables|Default|GetB1A%20S) (Variables|Default|GetB1A%20T) (Variables|Default|GetB2A%20S) (Variables|Default|GetB2A%20T) (== (Math|Float|Absolute(Float) (.x (Math|Vector|Normalize (Math|Vector|GetRightVector (Variables|Default|GetDefaultSceneRoot)) 1.0))) 0.0))))))))))))
    (else
      (Development|PrintString "Hello"))))

(event EventBeginPlay)

(event Collision|EventActorBeginOverlap
  (params (OtherActor :type Actor%20Object%20Reference)))

(event EventTick
  (params (DeltaSeconds :type Float%20%28single-precision%29)))

(fn ConstructionScript)