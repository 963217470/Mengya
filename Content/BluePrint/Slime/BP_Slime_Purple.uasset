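; BP_Slime_Purple is a child slime Blueprint whose merges add to an energy coefficient.
; MergeEffect calls the parent logic, then adds Param to EnergyCoefficient, while MergeTwice performs the same addition alone.
; Tick calls the parent, then writes EnergyValue and EnergyCoefficient as joined text to its W_Energy widget in dark grey, refreshing every frame.
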(event EventBeginPlay
  (|CallParentFunction) ; 此节点被禁用，将不会被调用。\n从引脚连出引线来编译功能。
)

(event Collision|EventActorBeginOverlap
  (params (OtherActor :type Actor%20Object%20Reference))
  (|CallParentFunction OtherActor) ; 此节点被禁用，将不会被调用。\n从引脚连出引线来编译功能。
)

(event EventTick
  (params (DeltaSeconds :type Float%20%28single-precision%29))
  (|CallParentFunction DeltaSeconds)
  (bind _asw_energy (Utilities|Casting|CastToW_Energy (UserInterface|GetWidget (Variables|Default|GetWidget))))
  (Default|SetTextandColor _asw_energy (Utilities|Text|ToText(String) (Utilities|String|Append (Utilities|String|ToString(Integer) (Variables|Default|GetEnergyValue)) "  " (Utilities|String|ToString(Float) (Variables|Default|GetEnergyCoefficient)))) "(R=0.250000,G=0.250000,B=0.250000,A=1.000000)"))

(fn ConstructionScript
  (|CallParentFunction))

(fn MergeTwice
  (params (Param :type Float%20%28double-precision%29))
  (Variables|Default|SetEnergyCoefficient (+ Param (Variables|Default|GetEnergyCoefficient))))

(fn MergeEffect
  (params (EffectItem :type Integer) (Param :type Float%20%28double-precision%29))
  (|CallParentFunction EffectItem Param)
  (Variables|Default|SetEnergyCoefficient (+ Param (Variables|Default|GetEnergyCoefficient)))
  (return))