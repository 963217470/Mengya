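; BP_Slime is a slime piece on a tile grid that holds an energy value, shown on its widget every tick.
; It provides timeline-driven move, move-then-destroy and merge-pulse events, plus surge effects and a one-time power-of-four energy check.
; FindNeighbor gets four-way adjacent slimes via index math on BP_SceneBox's tile array and box overlaps.
; It binds to BP_SceneBox's turn event, but TurnAlternation is empty.
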(event Custom|TurnAlternationEvent
  (CallFunction|TurnAlternation))

(event Custom|OnClicked_Event
  (params (TouchedActor :type Actor%20Object%20Reference) (ButtonPressed :type Key%20Structure :default "None"))
  (bind _neighbors (CallFunction|FindNeighbor))
  (bind _result (Utilities|Set|ToArray _neighbors))
  (for _array_element _result
    (Development|PrintString (Utilities|GetDisplayName _array_element) true true "(R=0.000000,G=0.660000,B=1.000000,A=1.000000)" 2.0 (Utilities|String|StringToName (Utilities|GetDisplayName _array_element)))))

(event Custom|MoveToDestroy
  (params (NewLocation :type Vector%20%28by%20ref%29) (Duration :type Float%20%28single-precision%29))
  (Utilities|FlowControl|Delay Duration)
  (bind _output_get (Variables|Default|SetOldLocation (Transformation|GetActorLocation)))
  (bind _floor (Timeline|move_to_delay时间轴 PlayFromStart)
    (:Update
      (Transformation|SetActorLocation (Math|Vector|Lerp(Vector) _output_get NewLocation _floor) false false))
    (:Finished
      (Actor|DestroyActor))))

(event Custom|MoveTo
  (params (NewLocation :type Vector))
  (bind _output_get (Variables|Default|SetOldLocation (Transformation|GetActorLocation)))
  (bind _floor (Timeline|move_to时间轴 PlayFromStart)
    (:Update
      (Transformation|SetActorLocation (Math|Vector|Lerp(Vector) _output_get NewLocation _floor) false false))))

(event Custom|MergeEvent
  (params (Scale :type Vector))
  (bind _skeletalmesh (Variables|Default|GetSkeletalMesh))
  (bind _returnvalue (Transformation|GetWorldLocation _skeletalmesh))
  (Utilities|FlowControl|Sequence
    (:then_0
      (goto _label Reset))
    (:then_1
      (Utilities|FlowControl|Delay 0.1)
      (bind _floor (Timeline|merge_event时间轴 PlayFromStart)
        (:Update
          (Transformation|SetWorldScale3D (Variables|Default|GetSkeletalMesh) (Math|Vector|Lerp(Vector) Scale (* Scale 1.5) _floor)))
        (:Finished
          (Utilities|FlowControl|DoOnce false :!label _label
            (:Completed
              (Niagara|SpawnSystematLocation (Variables|Default|GetSystem%20Template) (Math|Vector|MakeVector (.x _returnvalue) (.y _returnvalue) (+ (.z _returnvalue) 5e+01)) "0, 0, 0" (Math|Conversions|ToVector(Float) (Math|Float|Floor 1e+01)))
              (Timeline|merge_event时间轴 ReverseFromEnd))))))))

(event EventBeginPlay
  (bind _skeletalmesh (Variables|Default|GetSkeletalMesh))
  (Variables|Default|SetSk_Scale (Transformation|GetWorldScale _skeletalmesh))
  (Rendering|ToggleVisibility _skeletalmesh false)
  (if (Variables|Default|GetBirthOrMerge)
    _
    (else
      (Utilities|FlowControl|Delay 0.15)))
  (Rendering|ToggleVisibility _skeletalmesh false)
  (if (Variables|Default|GetBirthOrMerge)
    (Components|Animation|PlayAnimation (Variables|Default|GetSkeletalMesh) "/Game/BluePrint/Slime/SlimeAnimation/AM_Slime_Birth.AM_Slime_Birth" false))
  (bind _returnvalue (Actor|GetActorOfClass "/Game/BluePrint/Scene/BP_SceneBox.BP_SceneBox_C"))
  (EventDispatchers|BindEventtoTurnAlternation _returnvalue (delegate Custom|TurnAlternationEvent)))

(event Collision|EventActorBeginOverlap
  (params (OtherActor :type Actor%20Object%20Reference)))

(event EventTick
  (params (DeltaSeconds :type Float%20%28single-precision%29))
  (bind _asw_energy (Utilities|Casting|CastToW_Energy (UserInterface|GetWidget (Variables|Default|GetWidget))))
  (Default|SetTextandColor _asw_energy (Utilities|Text|ToText(Integer) (Variables|Default|GetEnergyValue)) "(R=0.250000,G=0.250000,B=0.250000,A=1.000000)"))

(fn ConstructionScript)

(fn MergeTwice
  (params (Param :type Float%20%28double-precision%29))
  (return))

(fn EnergySurge
  (Variables|Default|SetEnergyValue (* (Variables|Default|GetEnergyValue) 2))
  (return))

(fn ExplosionSurge
  (Actor|DestroyActor))

(fn MergeEffect
  (params (EffectItem :type Integer) (Param :type Float%20%28double-precision%29))
  (switch int EffectItem
    (:Default
      (return))
    (:0
      (Variables|Default|SetEnergyCoefficient (* (Variables|Default|GetEnergyCoefficient) 2.0)))))

(fn TurnAlternation
  (return))

(fn FindNeighbor
  (Utilities|Set|Clear (LocalVariables|Getneighbor_S))
  (Utilities|Array|Clear (LocalVariables|Getneighbor_T))
  (|FindTileN
    (:Completed
      (if (Utilities|Array|IsNotEmpty (LocalVariables|Getneighbor_T))
        (for _array_element (LocalVariables|Getneighbor_T)
          (if (Utilities|Array|IsNotEmpty (Collision|GetOverlappingActors (Variables|/Game/BluePrint/Scene/BP_FloorTile.BP_FloorTile_C|GetBox _array_element) "BP_Slime_C" :!class /Script/Engine.PrimitiveComponent))
            (bind _asbp_slime (Utilities|Casting|CastToBP_Slime (Utilities|Array|Get(acopy) (Collision|GetOverlappingActors (Variables|/Game/BluePrint/Scene/BP_FloorTile.BP_FloorTile_C|GetBox _array_element) "BP_Slime_C" :!class /Script/Engine.PrimitiveComponent))))
            (Utilities|Set|Add (LocalVariables|Getneighbor_S) _asbp_slime)))
        (return (LocalVariables|Getneighbor_S))))))

(fn Merge
  (Audio|SpawnSound2D "/Game/Sound/merge.merge" 1.0 1.0 0.0 0 false false)
  (CallFunction|MergeEvent (Variables|Default|GetSk_Scale))
  (return))

(fn Firstat4N
  (bind _energyvalue (Variables|Default|GetEnergyValue))
  (bind _returnvalue (Math|Conversions|ToFloat(Integer) _energyvalue))
  (bind _returnvalue_2 (Math|Float|Log _returnvalue 4.0))
  (if (Variables|Default|GetisAt4^n)
    (return false 0)
    (elif (and (!= _returnvalue_2 0.0) (== (Math|Float|%(Float) _returnvalue_2 1.0) 0.0))
      (Variables|Default|SetisAt4^n true)
      (return true (/ (Variables|Default|GetEnergyValue) 2))
      (else
        (return false 0)))))