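; BP_Slime_Red is a slime Blueprint that acts as a countdown bomb in a turn-based merge mechanic.
; Each turn and each energy surge lowers the countdown, while merge effects either extend it by a log2 of energy value or shorten it.
; When the turn decrement exhausts the countdown, it calls ExplosionSurge on its neighbors and then itself.
; Tick writes energy and countdown into its W_Energy widget.
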(event EventBeginPlay
  (|CallParentFunction) ; 此节点被禁用，将不会被调用。\n从引脚连出引线来编译功能。
)

(event Collision|EventActorBeginOverlap
  (params (OtherActor :type Actor%20Object%20Reference))
  (|CallParentFunction OtherActor) ; 此节点被禁用，将不会被调用。\n从引脚连出引线来编译功能。
)

(event EventTick
  (params (DeltaSeconds :type Float%20%28single-precision%29))
  (bind _asw_energy (Utilities|Casting|CastToW_Energy (UserInterface|GetWidget (Variables|Default|GetWidget))))
  (Default|SetText _asw_energy (Utilities|Text|ToText(String) (Utilities|String|Append (Utilities|String|ToString(Integer) (Variables|Default|GetEnergyValue)) "  " (Utilities|String|ToString(Integer) (Variables|Default|GetCountdown))))))

(fn ConstructionScript
  (|CallParentFunction))

(fn MergeEffect
  (params (EffectItem :type Integer) (Param :type Float%20%28double-precision%29))
  (|CallParentFunction EffectItem 0.0)
  (switch int EffectItem
    (:1
      (Variables|Default|SetCountdown (+ (Variables|Default|GetCountdown) (* (Math|Float|Log (Math|Conversions|ToFloat(Integer) (Variables|Default|GetEnergyValue)) 2.0) 3.0))))
    (:2
      (Variables|Default|SetCountdown (- (Variables|Default|GetCountdown) 3)))))

(fn TurnAlternation
  (|CallParentFunction)
  (bind _result (Math|Integer|DecrementInt (Variables|Default|GetCountdown))
    (:%20%20
      (if (<= _result 0)
        (bind _neighbors (CallFunction|FindNeighbor))
        (bind _result_2 (Utilities|Set|ToArray _neighbors))
        (for _array_element _result_2
          (Default|ExplosionSurge _array_element))
        (CallFunction|ExplosionSurge)))))

(fn EnergySurge
  (|CallParentFunction)
  (Math|Integer|DecrementInt (Variables|Default|GetCountdown)))